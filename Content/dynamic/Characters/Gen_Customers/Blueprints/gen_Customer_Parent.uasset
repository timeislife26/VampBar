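; Parent Blueprint for generated customers, giving each one a patience value that drains over time.
; On BeginPlay it passes itself to the Patience_Meter widget in its PatienceMeter component as OwnerBP.
; A looping timer, rather than Tick, lowers PatienceAmt in small steps and clears itself once patience runs out, with no further consequence here.
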(event `self.ReceiveBeginPlay`
  (`self.PatienceMeterFunction`)
  (bind _returnvalue (`KismetSystemLibrary.K2_SetTimerDelegate` (delegate `DeductPatience`) 0.1 true)))

(event `DeductPatience`
  (set `self.PatienceAmt` (- (`self.PatienceAmt`) 0.01))
  (if (<= (`self.PatienceAmt`) 0.0)
    (`KismetSystemLibrary.K2_ClearAndInvalidateTimerHandle` (stale `self.ReceiveBeginPlay` _returnvalue))))

(fn `PatienceMeterFunction`
  (bind _aspatience_meter (cast `/Game/dynamic/Characters/Gen_Customers/Widgets/Patience_Meter` (`WidgetComponent.GetWidget` (`self.PatienceMeter`))))
  (set `/Game/dynamic/Characters/Gen_Customers/Widgets/Patience_Meter.Owner_BP` self _aspatience_meter))

(fn `UserConstructionScript`)